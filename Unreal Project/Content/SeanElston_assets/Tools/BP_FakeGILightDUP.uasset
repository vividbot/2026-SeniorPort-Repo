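; Fake GI light tool that uses an emissive mesh card as a Lumen light source, configured entirely in the construction script.
; MaterialDefault applies MM_FakeGILight to LightMesh and passes color, temperature and intensity through default Custom Primitive Data, avoiding dynamic material instances.
; When SetSceneCaptureOnly is true, GeometrySetup hides the mesh in game while enabling its distance field lighting and ray tracing visibility.
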(event EventBeginPlay)

(event Collision|EventActorBeginOverlap
  (params (OtherActor :type Actor%20Object%20Reference)))

(event EventTick
  (params (DeltaSeconds :type Float%20%28single-precision%29)))

(fn ConstructionScript
  (Utilities|FlowControl|Sequence
    (:then_0
      (CallFunction|MaterialDefault))
    (:then_1
      (CallFunction|GeometrySetup))))

(fn MaterialDefault
  (bind _lightmesh (Variables|Default|GetLightMesh))
  (bind _gi_card_emissive_color (Variables|GILightColorandIntensity|GetGi%20Card%20Emissive%20Color))
  (bind _returnvalue (Math|Conversions|ToLinearColor(Color) _gi_card_emissive_color))
  (bind (_r _g _b) (Math|Color|BreakColor _returnvalue))
  (Rendering|Material|SetMaterial _lightmesh 0 "/Game/SeanElston_assets/Tools/MM_FakeGILight.MM_FakeGILight")
  (Rendering|Material|SetVectorParameterforDefaultCustomPrimitiveData _lightmesh "LumenLightColor" (Math|Vector4|MakeVector4 _r _g _b (Variables|GILightColorandIntensity|GetGI%20Card%20Color%20Temp)))
  (Class|PrimitiveComponent|SetScalarParameterforDefaultCustomPrimitiveData _lightmesh "LumenLightIntensity" (Variables|GILightColorandIntensity|GetGI%20Card%20Emissive%20Intensity)))

(fn GeometrySetup
  (bind _lightmesh (Variables|Default|GetLightMesh))
  (if (Variables|Default|GetSet%20Scene%20Capture%20Only)
    (Development|SetHiddeninGame _lightmesh true false)
    (Rendering|SetAffectDistanceFieldLighting _lightmesh true)
    (Class|PrimitiveComponent|SetVisibleinRayTracing _lightmesh true)))