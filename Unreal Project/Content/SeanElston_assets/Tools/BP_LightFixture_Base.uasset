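; BP_LightFixture_Base is a base light fixture actor that configures a point light and optional fixture mesh in its construction script.
; It applies intensity, temperature and attenuation radius from variables.
; With AssignRandomColors on, it sets light color from a lerp of Color and random RGB, saving it back; otherwise the color setter is unconnected.
; Unless hidden, the mesh is added dynamically with shadow settings and per-slot materials.
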(event EventBeginPlay)

(event Collision|EventActorBeginOverlap
  (params (OtherActor :type Actor%20Object%20Reference)))

(event EventTick
  (params (DeltaSeconds :type Float%20%28single-precision%29)))

(fn ConstructionScript
  (Utilities|FlowControl|Sequence
    (:then_0
      (CallFunction|LightValue))
    (:then_1
      (CallFunction|TempValue))
    (:then_2
      (CallFunction|ColorValue))
    (:then_3
      (CallFunction|Radius))
    (:then_4
      (CallFunction|CreateStaticMeshComponent))))

(fn CreateStaticMeshComponent
  (if (and (not (Variables|Default|GetHide%20SStatic%20Mesh)) (Utilities|IsValid (Variables|Default|GetLight%20Fixture%20Mesh)))
    (bind _returnvalue (AddComponent|AddStaticMeshComponent false (Variables|Default|GetRelative%20Transform)))
    (bind _output_get (Variables|Default|SetLight%20Fixture%20Mesh%20Component _returnvalue))
    (Utilities|IsValid _output_get
      (:Is%20Valid
        (Components|StaticMesh|SetStaticMesh _output_get (Variables|Default|GetLight%20Fixture%20Mesh))
        (Rendering|SetCastShadow _output_get (Variables|Default|GetStatic%20Mesh%20Cast%20Shadow))
        (Class|PrimitiveComponent|SetCastContactShadow _output_get (Variables|Default|GetStatic%20Mesh%20Contact%20Shadows))
        (for (_array_element _array_index) (Variables|Default|GetLight%20Fixture%20Mesh%20Material)
          (Rendering|Material|SetMaterial (Variables|Default|GetLight%20Fixture%20Mesh%20Component) _array_index _array_element)))
      (:Is%20Not%20Valid
        (Rendering|Material|SetMaterial (Variables|Default|GetLight%20Fixture%20Mesh%20Component) _array_index _array_element)))))

(fn LightValue
  (bind _output_get (Variables|Default|SetLight%20Intensity (Variables|Default|GetLight%20Intensity)))
  (Rendering|Components|Light|SetIntensity (Variables|Default|GetPointLight) _output_get))

(fn TempValue
  (bind _output_get (Variables|Default|SetTemp%20Kelvin (Variables|Default|GetTemp%20Kelvin)))
  (Class|LightComponent|SetTemperature (Variables|Default|GetPointLight) _output_get))

(fn ColorValue
  (bind _color_range_min (Variables|Default|GetColor%20Range%20Min))
  (bind _color_range_max (Variables|Default|GetColor%20Range%20Max))
  (bind _pointlight (Variables|Default|GetPointLight))
  (if (Variables|Default|GetAssign%20Random%20Colors)
    (Rendering|Components|Light|SetLightColor _pointlight (Class|KismetMathLibrary|HSVtoRGBLinear (Class|KismetMathLibrary|RGBLineartoHSV (Math|Color|Lerp(LinearColor) (Variables|Default|GetColor) (Utilities|Struct|MakeLinearColor (Math|Random|RandomFloatinRange _color_range_min _color_range_max) (Math|Random|RandomFloatinRange _color_range_min _color_range_max) (Math|Random|RandomFloatinRange _color_range_min _color_range_max) 1.0) 0.0))) true)
    (Variables|Default|SetColor (Rendering|Components|Light|GetLightColor _pointlight))
    (else
      (bind _output_get (Variables|Default|SetColor (Variables|Default|GetColor))))))

(fn Radius
  (bind _output_get (Variables|Default|SetRadius%20Value (Variables|Default|GetRadius%20Value)))
  (Rendering|Lighting|SetAttenuationRadius (Variables|Default|GetPointLight) _output_get))